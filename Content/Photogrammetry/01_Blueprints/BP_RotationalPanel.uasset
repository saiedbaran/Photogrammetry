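; BP_RotationalPanel is a photogrammetry turntable that spins an attached actor and takes screenshots at regular angular steps.
; BeginPlay attaches AttachedActor, then Tick yaws the panel at Speed while the device is on and rotation is enabled, tracking accumulated angle.
; Each time RotationSteps is reached, OnCapture pauses rotation, runs the HighResShot console command, and resumes after a delay.
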(event Custom|OnCapture
  (Variables|Default|SetbEnableRotation false)
  (Development|ExecuteConsoleCommand "HighResShot 1920x1080" (Game|GetPlayerController 0))
  (Utilities|FlowControl|Delay (Variables|Default|GetDelay))
  (Variables|Default|SetbEnableRotation true))

(event EventBeginPlay
  (bind _attachedactor (Variables|Default|GetAttachedActor))
  (Utilities|IsValid _attachedactor
    (:Is%20Valid
      (Transformation|AttachActorToActor _attachedactor self "None" "KeepWorld" "KeepWorld" "KeepWorld" true))))

(event Collision|EventActorBeginOverlap
  (params (OtherActor :type Actor%20Object%20Reference)))

(event EventTick
  (params (DeltaSeconds :type Float%20%28single-precision%29))
  (bind _speed (Variables|Default|GetSpeed))
  (bind _returnvalue (* DeltaSeconds _speed))
  (if (Variables|Default|Getb_DeviceIsOn)
    (if (Variables|Default|GetbEnableRotation)
      (Variables|Default|SetRotationValue (+ _returnvalue (Variables|Default|GetRotationValue)))
      (Class|Actor|AddActorWorldRotation (Math|Rotator|MakeRotator 0.0 0.0 _returnvalue))
      (if (>= (- (Variables|Default|GetRotationValue) (Variables|Default|GetSavedRotation)) (Variables|Default|GetRotation%20Steps))
        (Variables|Default|SetSavedRotation (Variables|Default|GetRotationValue))
        (CallFunction|OnCapture)
        (else
          (Development|PrintString (Utilities|String|ToString(Float) (- (Variables|Default|GetRotationValue) (Variables|Default|GetSavedRotation))) true true "(R=0.000000,G=0.660000,B=1.000000,A=1.000000)" 0.01))))))

(fn ConstructionScript)